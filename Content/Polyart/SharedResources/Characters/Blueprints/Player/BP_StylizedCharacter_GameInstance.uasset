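; Game instance for the stylized character that owns the BP_SaveGame object and persists color sets to a save slot.
; On Init it synchronously loads the slot or creates a new save object; only successful async loads fire OnGameLoaded.
; Add, remove and modify events forward to the save object, then write it, asynchronously for remove and modify.
; Getter functions expose the save data and color set lookups.
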(event EventInit
  (CallFunction|LoadGameData false))

(event EventSaveGameData
  (params (Async :type Boolean))
  (bind _slot_name (Variables|Default|GetSlot%20Name))
  (bind _save_data (Variables|Default|GetSave%20Data))
  (if Async
    (|AsyncSaveGametoSlot _save_data _slot_name)
    (else
      (SaveGame|SaveGametoSlot _save_data _slot_name))))

(event EventLoadGameData
  (params (Async :type Boolean))
  (bind _returnvalue (SaveGame|DoesSaveGameExist (Variables|Default|GetSlot%20Name)))
  (if _returnvalue
    (if Async
      (bind _savegame (|AsyncLoadGamefromSlot (Variables|Default|GetSlot%20Name))
        (:Completed
          (bind _asbp_save_game (Utilities|Casting|CastToBP_SaveGame _savegame))
          (Variables|Default|SetSave%20Data _asbp_save_game)
          (Default|CallOnGameLoaded)))
      (else
        (bind _returnvalue_2 (SaveGame|LoadGamefromSlot (Variables|Default|GetSlot%20Name)))
        (bind _asbp_save_game_2 (Utilities|Casting|CastToBP_SaveGame _returnvalue_2))
        (Variables|Default|SetSave%20Data _asbp_save_game_2)))
    (else
      (bind _returnvalue_3 (SaveGame|CreateSaveGameObject "/Game/Polyart/SharedResources/Characters/Blueprints/SaveAndLoad/BP_SaveGame.BP_SaveGame_C"))
      (Variables|Default|SetSave%20Data _returnvalue_3))))

(event EventSaveColorSet
  (params (Color%20Set :type F%20Color%20Set%20Structure) (Async :type Boolean))
  (Default|AddColorSet (Variables|Default|GetSave%20Data) Color%20Set)
  (CallFunction|SaveGameData Async))

(event EventRemoveColorfromSet
  (params (Color%20Set :type Text) (Color :type Linear%20Color%20Structure))
  (Default|RemoveColorfromColorSet (Variables|Default|GetSave%20Data) Color%20Set Color)
  (CallFunction|SaveGameData true))

(event EventModifyColorinSet
  (params (Color%20Set%20Name :type Text) (Category%20%28optional%29 :type String) (Previous%20Color :type Linear%20Color%20Structure) (New%20Param :type F%20Color%20System%20Param%20Structure))
  (Default|ModifyColorinSet (Variables|Default|GetSave%20Data) Color%20Set%20Name Category%20%28optional%29 Previous%20Color New%20Param)
  (CallFunction|SaveGameData true))

(fn GetColorfromSetbyIndex
  (params (Color%20Set :type F%20Color%20Set%20Structure) (Index :type Integer))
  (bind _parameters (Utilities|Struct|BreakF_ColorSet Color%20Set))
  (if (Utilities|Array|IsValidIndex _parameters Index)
    (return (Utilities|Array|Get(acopy) _parameters Index))
    (else
      (return (Utilities|Struct|MakeF_ColorSystemParam "(R=0.000000,G=0.000000,B=0.000000,A=1.000000)" (Utilities|Array|MakeArray "") (Utilities|Array|MakeArray ""))))))

(fn GetColorParamsfromSet
  (params (Color%20Name :type Text) (Category%20%28optional%29 :type String) (Color :type Linear%20Color%20Structure))
  (bind _save_data (Variables|Default|GetSave%20Data))
  (bind (_found_ _params) (Default|GetColorParamsfromSet _save_data Color%20Name Category%20%28optional%29 Color))
  (return _found_ _params))

(fn GetColorSet
  (params (Color%20Set%20Name :type Text) (Category%20%28optional%29 :type String))
  (bind _save_data (Variables|Default|GetSave%20Data))
  (bind (_exists_ _out_color_set) (Default|ColorSetExists? _save_data Color%20Set%20Name Category%20%28optional%29))
  (Utilities|IsValid _save_data
    (:Is%20Valid
      (if _exists_
        (return true _out_color_set)
        (else
          _)))
    (:Is%20Not%20Valid
      (Development|PrintString "Save Data is not Valid")))
  (return false ""))

(fn GetColorSetsfromCategory
  (params (Category :type String))
  (bind _color_sets (Default|GetColorSetsfromCategory (Variables|Default|GetSave%20Data) Category))
  (return _color_sets))

(fn GetGameData
  (return (Variables|Default|GetSave%20Data)))

(fn GetAllColorSets
  (return (Variables|/Game/Polyart/SharedResources/Characters/Blueprints/SaveAndLoad/BP_SaveGame.BP_SaveGame_C|GetColor%20Sets (Variables|Default|GetSave%20Data))))