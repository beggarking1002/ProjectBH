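; BI_SaveGame is a Blueprint interface for saving and loading game data, with a focus on saved color sets used by Polyart characters.
; It declares load, save and get calls for game data, with an async option on loading, saving and saving color sets.
; Color set functions add, fetch, edit and remove colors, querying by name, optional category or index.
; It holds only signatures, leaving implementation to whichever class implements it.
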(fn LoadGameData
  (params (Async :type Boolean)))

(fn SaveGameData
  (params (Async :type Boolean)))

(fn GetGameData
  (return 0))

(fn SaveColorSet
  (params (Color%20Set :type F%20Color%20Set%20Structure) (Async :type Boolean)))

(fn GetColorSet
  (params (Color%20Set%20Name :type Text) (Category%20%28optional%29 :type String))
  (return false ""))

(fn RemoveColorfromSet
  (params (Color%20Set :type Text) (Color :type Linear%20Color%20Structure)))

(fn GetColorSetsfromCategory
  (params (Category :type String))
  (return 0))

(fn ModifyColorinSet
  (params (Color%20Set%20Name :type Text) (Category%20%28optional%29 :type String) (Previous%20Color :type Linear%20Color%20Structure) (New%20Param :type F%20Color%20System%20Param%20Structure)))

(fn GetColorParamsfromSet
  (params (Color%20Name :type Text) (Category%20%28optional%29 :type String) (Color :type Linear%20Color%20Structure))
  (return false ""))

(fn GetAllColorSets
  (return 0))

(fn GetColorfromSetbyIndex
  (params (Color%20Set :type F%20Color%20Set%20Structure) (Index :type Integer))
  (return ""))