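; Inventory component that tracks backpack ownership and decides whether its owner can pick up items.
; Pickup is allowed only with a backpack and while the held item count is below backpack capacity.
; On BeginPlay a looping timer delays caching the owner reference, then clears itself on its first call.
; A getter and setter expose the backpack flag; no logic here adds or removes items.
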(event EventBeginPlay
  (Utilities|Time|SetTimerbyFunctionName 0 "Set Initial References" 0.3 true))

(fn CanPickUp?
  (return (and (Variables|Backpack|GetHasBackpack?) (< (Utilities|Array|Length (Variables|Inventory|GetHeld%20Items)) (Variables|Backpack|GetBackpack%20Capacity)))))

(fn SetInitialReferences
  (Variables|References|SetOwner (Components|GetOwner))
  (Utilities|Time|ClearTimerbyFunctionName 0 "Set Initial References"))

(fn GetHasBackpack
  (return (Variables|Backpack|GetHasBackpack?)))

(fn SetHasBackpack
  (params (HasBackpack? :type Boolean))
  (Variables|Backpack|SetHasBackpack? HasBackpack?))