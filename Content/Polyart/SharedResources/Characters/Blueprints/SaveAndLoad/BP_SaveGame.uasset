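; Save game object that stores named, categorized color sets, apparently for character customization, and provides functions to query and edit them.
; ColorSetExists looks sets up by name and optional category; adding a set that already exists appends its parameters to the stored one.
; Individual colors are matched by display color with a small tolerance.
; Edits rebuild the set struct, add it to the array and remove the old entry, so edited sets change order.
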(fn ColorSetExists?
  (params (Color%20Set%20Name :type Text%20%28by%20ref%29) (Category%20%28optional%29 :type String))
  (for _array_element (Variables|Default|GetColor%20Sets)
    (if (and (Utilities|Enum|Equal(Enum) (.ColorSetName (Utilities|Struct|BreakF_ColorSet _array_element)) Color%20Set%20Name) (or (Utilities|Enum|Equal(Enum) (.Category (Utilities|Struct|BreakF_ColorSet _array_element)) Category%20%28optional%29) (Utilities|Array|IsEmpty Category%20%28optional%29)))
      (return true _array_element)))
  (return false ""))

(fn AddColorSet
  (params (In%20Color%20Set :type F%20Color%20Set%20Structure))
  (bind (_colorsetname _parameters _optionalfiltertag _category) (Utilities|Struct|BreakF_ColorSet In%20Color%20Set))
  (bind (_exists_ _out_color_set) (CallFunction|ColorSetExists? _colorsetname _category))
  (bind (_colorsetname_2 _parameters_2 _optionalfiltertag_2 _category_2) (Utilities|Struct|BreakF_ColorSet _out_color_set))
  (if _exists_
    (bind _output_get (LocalVariables|SetTemp%20Array _parameters_2))
    (Utilities|Array|AppendArray _output_get _parameters)
    (Utilities|Array|Add (Variables|Default|GetColor%20Sets) (Utilities|Struct|MakeF_ColorSet _colorsetname_2 (LocalVariables|GetTemp%20Array) _optionalfiltertag_2 _category_2))
    (Utilities|Array|RemoveItem (Variables|Default|GetColor%20Sets) _out_color_set)
    (else
      (Utilities|Array|Add (Variables|Default|GetColor%20Sets) In%20Color%20Set))))

(fn RemoveColorfromColorSet
  (params (Color%20Set%20Name :type Text%20%28by%20ref%29) (Color :type Linear%20Color%20Structure))
  (bind (_exists_ _out_color_set) (CallFunction|ColorSetExists? Color%20Set%20Name))
  (if _exists_
    (LocalVariables|SetFound%20Color%20Set _out_color_set)
    (bind _output_get (LocalVariables|SetTemp%20Array (.parameters (LocalVariables|GetFound%20Color%20Set))))
    (for (_array_element _array_index) _output_get
      (if (Class|KismetMathLibrary|LinearColorIsNearEqual (.DisplayColor (Utilities|Struct|BreakF_ColorSystemParam _array_element)) Color 0.001)
        (Utilities|Array|RemoveIndex (LocalVariables|GetTemp%20Array) _array_index)
        (Utilities|Array|Add (Variables|Default|GetColor%20Sets) (Utilities|Struct|MakeF_ColorSet (.colorsetname (LocalVariables|GetFound%20Color%20Set)) (LocalVariables|GetTemp%20Array) (.optionalfiltertag (LocalVariables|GetFound%20Color%20Set)) (.category (LocalVariables|GetFound%20Color%20Set))))
        (Utilities|Array|RemoveItem (Variables|Default|GetColor%20Sets) (LocalVariables|GetFound%20Color%20Set))
        (return)))))

(fn GetColorSetsfromCategory
  (params (Category :type String%20%28by%20ref%29))
  (for _array_element (Variables|Default|GetColor%20Sets)
    (if (Utilities|Enum|Equal(Enum) (.Category (Utilities|Struct|BreakF_ColorSet _array_element)) Category)
      (Utilities|Array|Add (LocalVariables|GetTemp%20Array) _array_element)))
  (return (LocalVariables|GetTemp%20Array)))

(fn ModifyColorinSet
  (params (Color%20Set%20Name :type Text) (Category%20%28optional%29 :type String) (Prev%20Color :type Linear%20Color%20Structure) (New%20Param :type F%20Color%20System%20Param%20Structure))
  (bind (_exists_ _out_color_set) (CallFunction|ColorSetExists? Color%20Set%20Name Category%20%28optional%29))
  (if _exists_
    (LocalVariables|SetFound%20Color%20Set _out_color_set)
    (bind _output_get (LocalVariables|SetTemp%20Array (.parameters (LocalVariables|GetFound%20Color%20Set))))
    (for (_array_element _array_index) _output_get
      (if (Class|KismetMathLibrary|LinearColorIsNearEqual (.DisplayColor (Utilities|Struct|BreakF_ColorSystemParam _array_element)) Prev%20Color 0.001)
        (Utilities|Array|SetArrayElem (LocalVariables|GetTemp%20Array) _array_index New%20Param)
        (Utilities|Array|Add (Variables|Default|GetColor%20Sets) (Utilities|Struct|MakeF_ColorSet (.colorsetname (LocalVariables|GetFound%20Color%20Set)) (LocalVariables|GetTemp%20Array) (.optionalfiltertag (LocalVariables|GetFound%20Color%20Set)) (.category (LocalVariables|GetFound%20Color%20Set))))
        (Utilities|Array|RemoveItem (Variables|Default|GetColor%20Sets) (LocalVariables|GetFound%20Color%20Set))
        (return)))))

(fn GetColorParamsfromSet
  (params (Color%20Set%20Name :type Text) (Category%20%28optional%29 :type String) (Color :type Linear%20Color%20Structure))
  (bind (_exists_ _out_color_set) (CallFunction|ColorSetExists? Color%20Set%20Name Category%20%28optional%29))
  (if _exists_
    (for _array_element (.Parameters (Utilities|Struct|BreakF_ColorSet _out_color_set))
      (if (Class|KismetMathLibrary|LinearColorIsNearEqual (.DisplayColor (Utilities|Struct|BreakF_ColorSystemParam _array_element)) Color 0.001)
        (return true _array_element))))
  (return false ""))