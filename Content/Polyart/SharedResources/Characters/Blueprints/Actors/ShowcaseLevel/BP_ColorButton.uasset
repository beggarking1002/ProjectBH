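; Showcase-level button actor that randomizes the colors of a modular character held in its Character child actor whenever its begin-overlap event fires.
; A second after BeginPlay it caches the character's BPC_ModularParts, triggers both overlap events once, and changes gender if not male.
; RandomizeColors blocking-loads each available-colors data asset, appends randomly picked color and float params without clearing previous ones, then passes them to ChangeColors.
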(event EventBeginPlay
  (bind _character (Variables|Default|GetCharacter))
  (bind _childactor (Variables|/Script/Engine.ChildActorComponent|GetChildActor _character))
  (bind _returnvalue (Actor|GetComponentbyClass _childactor "/Game/Polyart/SharedResources/Characters/Blueprints/Components/BPC_ModularParts.BPC_ModularParts_C"))
  (|CallParentFunction)
  (Utilities|FlowControl|Delay 1.0)
  (Utilities|IsValid _returnvalue
    (:Is%20Valid
      (Variables|Default|SetBPC%20Modular%20Parts _returnvalue)
      (CallFunction|OnBeginOverlap)
      (CallFunction|OnEndOverlap)
      (if (not (Variables|Settings|GetIs%20Male?))
        (Default|ChangeGender (Variables|Default|GetBPC%20Modular%20Parts))))))

(event EventOnBeginOverlap
  (|CallParentFunction)
  (CallFunction|RandomizeColors))

(fn ConstructionScript
  (|CallParentFunction))

(fn RandomizeColors
  (Utilities|FlowControl|Sequence
    (:then_0
      (for _array_element (Variables|/Game/Polyart/SharedResources/Characters/DataAssets/BP_Data_Holder.BP_Data_Holder_C|GetArray (Variables|Default|GetDA%20Randomize%20Colors))
        (bind _returnvalue (Utilities|LoadAssetBlocking _array_element))
        (bind _aspda_available_colors (Utilities|Casting|CastToBP_Data_AvailableColors _returnvalue))
        (Utilities|Array|AppendArray (LocalVariables|GetColor%20Params) (.ColorParams (Utilities|Struct|BreakF_ColorSystemParam (Utilities|Array|Get(acopy) (.Parameters (Utilities|Struct|BreakF_ColorSet (Variables|/Game/Polyart/SharedResources/Characters/DataAssets/BP_Data_AvailableColors.BP_Data_AvailableColors_C|GetColor%20Sets _aspda_available_colors))) (Math|Random|RandomIntegerinRange 0 (- (Utilities|Array|Length (.Parameters (Utilities|Struct|BreakF_ColorSet (Variables|/Game/Polyart/SharedResources/Characters/DataAssets/BP_Data_AvailableColors.BP_Data_AvailableColors_C|GetColor%20Sets _aspda_available_colors)))) 1))))))
        (Utilities|Array|AppendArray (LocalVariables|GetFloat%20Params) (.FloatParams (Utilities|Struct|BreakF_ColorSystemParam (Utilities|Array|Get(acopy) (.Parameters (Utilities|Struct|BreakF_ColorSet (Variables|/Game/Polyart/SharedResources/Characters/DataAssets/BP_Data_AvailableColors.BP_Data_AvailableColors_C|GetColor%20Sets _aspda_available_colors))) (Math|Random|RandomIntegerinRange 0 (- (Utilities|Array|Length (.Parameters (Utilities|Struct|BreakF_ColorSet (Variables|/Game/Polyart/SharedResources/Characters/DataAssets/BP_Data_AvailableColors.BP_Data_AvailableColors_C|GetColor%20Sets _aspda_available_colors)))) 1))))))))
    (:then_1
      (Default|ChangeColors (Variables|Default|GetBPC%20Modular%20Parts) (LocalVariables|GetColor%20Params) (LocalVariables|GetFloat%20Params) (Utilities|Array|MakeArray "")))))