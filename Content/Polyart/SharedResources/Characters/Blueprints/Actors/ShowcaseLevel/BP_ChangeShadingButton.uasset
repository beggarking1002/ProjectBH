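; Showcase level button that, on overlap, switches the player character's shading between PBR and cel-shaded for demonstration.
; It overrides the parent's overlap handler and calls the shading change on the player pawn's BPC_ModularParts component.
; If the pawn has a valid backpack part component, it re-equips that part with male and female backpack meshes chosen by the component's UsePBR flag.
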(event EventBeginPlay
  (|CallParentFunction) ; This node is disabled and will not be called.\nDrag off pins to build functionality.
)

(event Collision|EventActorBeginOverlap
  (params (OtherActor :type Actor%20Object%20Reference))
  (|CallParentFunction OtherActor) ; This node is disabled and will not be called.\nDrag off pins to build functionality.
)

(event EventTick
  (params (DeltaSeconds :type Float%20%28single-precision%29))
  (|CallParentFunction DeltaSeconds) ; This node is disabled and will not be called.\nDrag off pins to build functionality.
)

(fn ConstructionScript
  (|CallParentFunction))

(fn OnBeginOverlap
  (bind _returnvalue (Game|Player|GetPlayerPawn 0))
  (bind _returnvalue_2 (Actor|GetComponentbyClass _returnvalue "/Game/Polyart/SharedResources/Characters/Blueprints/Components/BPC_ModularParts.BPC_ModularParts_C"))
  (|CallParentFunction)
  (Utilities|IsValid _returnvalue_2
    (:Is%20Valid
      (bind _output_get (LocalVariables|SetBPC%20Modular%20Parts _returnvalue_2))
      (Default|ChangeShading(ShowcasePurposes) _output_get)
      (Utilities|IsValid (Default|SelectPartbyEnum (LocalVariables|GetBPC%20Modular%20Parts) "NewEnumerator10")
        (:Is%20Valid
          (Default|EquipPart (LocalVariables|GetBPC%20Modular%20Parts) (Utilities|Struct|MakeF_ModularPart (select (Variables|/Game/Polyart/SharedResources/Characters/Blueprints/Components/BPC_ModularParts.BPC_ModularParts_C|GetUse%20PBR? (LocalVariables|GetBPC%20Modular%20Parts)) "/Game/Polyart/ModularStylizedChars/Meshes/SkeletalMeshes/Props/Backpack/SK_MaleBackpack.SK_MaleBackpack" "/Game/Polyart/ModularStylizedChars/Meshes/SkeletalMeshes/Props/Backpack/SK_MaleBackpackCelShaded.SK_MaleBackpackCelShaded") (select (Variables|/Game/Polyart/SharedResources/Characters/Blueprints/Components/BPC_ModularParts.BPC_ModularParts_C|GetUse%20PBR? (LocalVariables|GetBPC%20Modular%20Parts)) "/Game/Polyart/ModularStylizedChars/Meshes/SkeletalMeshes/Props/Backpack/SK_FemaleBackpack.SK_FemaleBackpack" "/Game/Polyart/ModularStylizedChars/Meshes/SkeletalMeshes/Props/Backpack/SK_FemaleBackpackCelShaded.SK_FemaleBackpackCelShaded") "NewEnumerator10" 0) "backpack" (Default|SelectPartbyEnum (LocalVariables|GetBPC%20Modular%20Parts) "NewEnumerator10")))))))