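; Pickable item actor whose Backpack component spins and bobs on a sine wave until picked up.
; When an actor with BPC_Inventory overlaps its sphere, CanPickUp selects one of two timeline-driven responses.
; Success plays once, spinning, scaling and moving the item toward the picker under a fresnel overlay, then destroys it.
; Refusal animates a sideways nudge from its initial location with a temporary red overlay.
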(event OnComponentBeginOverlap(Sphere)
  (params (OverlappedComponent :type Primitive%20Component%20Object%20Reference) (OtherActor :type Actor%20Object%20Reference) (OtherComp :type Primitive%20Component%20Object%20Reference) (OtherBodyIndex :type Integer) (bFromSweep :type Boolean) (SweepResult :type Hit%20Result%20Structure%20%28by%20ref%29))
  (bind _returnvalue (Actor|GetComponentbyClass OtherActor "/Game/Polyart/SharedResources/Characters/Blueprints/Components/BPC_Inventory.BPC_Inventory_C"))
  ;[0.07812 0.07812 0.07812] On try to pick up event
  (Utilities|IsValid _returnvalue
    (:Is%20Valid
      (Variables|References|SetPicker%20Actor OtherActor)
      (if (Default|CanPickUp? _returnvalue)
        (|HasBackpacLogic)
        (else
          (|NoBackpackLogic))))))

(event EventTick
  (params (DeltaSeconds :type Float%20%28single-precision%29))
  ;[0.05208 0.05208 0.05208] Default Rotation Animation
  (if (Variables|StoredVariables|GetIs%20NOT%20Picked%20Up?)
    (Transformation|AddLocalRotation (Variables|Default|GetBackpack) (Math|Rotator|MakeRotator 0.0 0.0 (Variables|AnimationSettings|GetRotation%20Speed)) false false)
    (Transformation|AddLocalOffset (Variables|Default|GetBackpack) (Math|Vector|MakeVector 0.0 0.0 (* (Math|Trig|Sin(Radians) (* (Utilities|Time|GetTimeSeconds) (Variables|AnimationSettings|GetMovement%20Speed))) (Variables|AnimationSettings|GetMovement%20Range))) false false)))

(fn ConstructionScript
  (Variables|StoredVariables|SetInitial%20Location (Transformation|GetActorLocation)))