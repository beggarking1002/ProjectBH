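; BP_Backpack is a world pickup that gives an overlapping character a backpack.
; On sphere overlap, it checks the actor's BPC_Inventory and, if no backpack is owned, sets the flag and adds a new skeletal mesh component.
; BPC_ModularParts then equips the male/female backpack part onto it, choosing PBR or cel-shaded meshes via UsePBR, and the pickup destroys itself.
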(event OnComponentBeginOverlap(Sphere)
  (params (OverlappedComponent :type Primitive%20Component%20Object%20Reference) (OtherActor :type Actor%20Object%20Reference) (OtherComp :type Primitive%20Component%20Object%20Reference) (OtherBodyIndex :type Integer) (bFromSweep :type Boolean) (SweepResult :type Hit%20Result%20Structure%20%28by%20ref%29))
  (bind _returnvalue (Actor|GetComponentbyClass OtherActor "/Game/Polyart/SharedResources/Characters/Blueprints/Components/BPC_Inventory.BPC_Inventory_C"))
  (bind _returnvalue_2 (Actor|GetComponentbyClass OtherActor "/Game/Polyart/SharedResources/Characters/Blueprints/Components/BPC_ModularParts.BPC_ModularParts_C"))
  (bind _use_pbr_ (Variables|/Game/Polyart/SharedResources/Characters/Blueprints/Components/BPC_ModularParts.BPC_ModularParts_C|GetUse%20PBR? _returnvalue_2))
  ;[0.04688 0.04688 0.04688] On try to pick up event
  (Utilities|IsValid _returnvalue
    (:Is%20Valid
      (if (not (Default|GetHasBackpack _returnvalue))
        (Default|SetHasBackpack _returnvalue true)
        (bind _returnvalue_3 (Game|AddComponentbyClass OtherActor "/Script/Engine.SkeletalMeshComponent" false))
        (Default|EquipPart _returnvalue_2 (Utilities|Struct|MakeF_ModularPart (select _use_pbr_ "/Game/Polyart/ModularStylizedChars/Meshes/SkeletalMeshes/Props/Backpack/SK_MaleBackpack.SK_MaleBackpack" "/Game/Polyart/ModularStylizedChars/Meshes/SkeletalMeshes/Props/Backpack/SK_MaleBackpackCelShaded.SK_MaleBackpackCelShaded") (select _use_pbr_ "/Game/Polyart/ModularStylizedChars/Meshes/SkeletalMeshes/Props/Backpack/SK_FemaleBackpack.SK_FemaleBackpack" "/Game/Polyart/ModularStylizedChars/Meshes/SkeletalMeshes/Props/Backpack/SK_FemaleBackpackCelShaded.SK_FemaleBackpackCelShaded") (Variables|Default|GetPart) 0) "Backpack" _returnvalue_3)
        (Actor|DestroyActor)))))

(fn ConstructionScript
  (Components|SkeletalMesh|SetSkeletalMeshAsset (Variables|Default|GetBackpack) (Variables|MeshSettings|GetMaleBackpack)))