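; Blueprint function library that maps a character body part to material parameter names and a filter tag, apparently for makeup customization.
; Pure lookups use Select nodes to return the color, intensity and makeup mask texture parameter names for each part.
; Face parts (eyes, mouth, face) and body parts (torso, arms, legs) reuse the same three mask channels, distinguished by a "face" or "body" tag.
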(fn GetColorPropertyName
  (params (Body%20Slot :type E_BodyPaintSlot%20Enum :default "NewEnumerator0"))
  (return (Utilities|Select :Index Body%20Slot :NewEnumerator0 "Mask 1 Color" :NewEnumerator1 "Mask 2 Color" :NewEnumerator2 "Mask 3 Color" :NewEnumerator3 "Mask 1 Color" :NewEnumerator4 "Mask 2 Color" :NewEnumerator5 "Mask 3 Color")))

(fn GetIntensityPropertyName
  (params (Body%20Part :type E_BodyPaintSlot%20Enum :default "NewEnumerator0"))
  (return (Utilities|Select :Index Body%20Part :NewEnumerator0 "Mask 1 Intensity" :NewEnumerator1 "Mask 2 Intensity" :NewEnumerator2 "Mask 3 Intensity" :NewEnumerator3 "Mask 1 Intensity" :NewEnumerator4 "Mask 2 Intensity" :NewEnumerator5 "Mask 3 Intensity")))

(fn GetTexturePropertyName
  (params (Body%20Part :type E_BodyPaintSlot%20Enum :default "NewEnumerator0"))
  (return (Utilities|Select :Index Body%20Part :NewEnumerator0 "Makeup Mask 1" :NewEnumerator1 "Makeup Mask 2" :NewEnumerator2 "Makeup Mask 3" :NewEnumerator3 "Makeup Mask 1" :NewEnumerator4 "Makeup Mask 2" :NewEnumerator5 "Makeup Mask 3")))

(fn GetOptionalFilterTag
  (params (Body%20Part :type E_BodyPaintSlot%20Enum :default "NewEnumerator0"))
  (return (Utilities|Select :Index Body%20Part :NewEnumerator0 "face" :NewEnumerator1 "face" :NewEnumerator2 "face" :NewEnumerator3 "body" :NewEnumerator4 "body" :NewEnumerator5 "body")))